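; Cine camera actor that renders a viewport capture to a render target through a Composure element it creates on BeginPlay.
; It gathers cameras of a target class, then each tick snaps to the one at CameraIndex, copying its capture settings and focal length.
; The vision actor and Rain-tagged actor follow the camera.
; When the index is invalid, it follows the player camera instead.
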(event EventBeginPlay
  (bind _returnvalue (Class|ComposureBlueprintLibrary|CreateComposureElement "ViewportCapture" "/Composure/Blueprints/CompositingElements/BP_CgCaptureCompElement.BP_CgCaptureCompElement_C" self))
  (bind _output_get (Variables|Default|SetCompEl _returnvalue))
  (Class|CompositingElement|SetTargetCamera _output_get self)
  (Class|ComposureBlueprintLibrary|RefreshComposureElementList)
  (bind _returnvalue_2 (Class|CompositingElement|CreateNewOutputPass (Variables|Default|GetCompEl) "OutputPass" "/Script/Composure.RenderTargetCompositingOutput"))
  (Variables|/Script/Composure.RenderTargetCompositingOutput|SetRenderTarget _returnvalue_2 "/ROSIntegrationVision/RT_ViewportCineCapture.RT_ViewportCineCapture")
  (Variables|/Script/Composure.CompositingElement|SetRenderResolution (Variables|Default|GetCompEl) (Utilities|Struct|MakeIntPoint 1920 1080))
  (Utilities|FlowControl|Delay 0.2)
  (bind _outactors (Actor|GetAllActorsOfClass (Variables|Default|GetTargetCameraClass)))
  (Variables|Default|SetAllCameras _outactors)
  (Variables|/Composure/Blueprints/CompositingElements/BP_CgCaptureCompElement.BP_CgCaptureCompElement_C|SetColorGradeSettings (Variables|Default|GetCompEl) (Utilities|Struct|MakeUDS_ColorGradeSettings "(R=1.000000,G=1.000000,B=1.000000,A=0.880000)" "(R=1.000000,G=1.000000,B=1.000000,A=0.880000)" "(R=1.000000,G=1.000000,B=1.000000,A=1.750000)" "(R=1.000000,G=1.000000,B=1.000000,A=0.880000)" "(R=0.000000,G=0.000000,B=0.000000,A=0.000000)")))

(event Collision|EventActorBeginOverlap
  (params (OtherActor :type Actor%20Object%20Reference)))

(event EventTick
  (params (DeltaSeconds :type Float%20%28single-precision%29))
  (bind _returnvalue (Game|GetPlayerCameraManager 0))
  (if (Utilities|Array|IsValidIndex (Variables|Default|GetAllCameras) (Variables|Default|GetCameraIndex))
    (Transformation|AttachActorToActor (Utilities|Array|Get(acopy) (Variables|Default|GetAllCameras) (Variables|Default|GetCameraIndex)) "None" "SnapToTarget" "SnapToTarget" "SnapToTarget" true)
    (Default|CopyCameraSettingstoSceneCapture (Variables|Default|GetCompEl) (Variables|/Script/Engine.CameraActor|GetCameraComponent (Utilities|Array|Get(acopy) (Variables|Default|GetAllCameras) (Variables|Default|GetCameraIndex))) (Variables|/Script/Composure.CompositingCaptureBase|GetSceneCaptureComponent2D (Variables|Default|GetCompEl)))
    (bind _ascine_camera_component (Utilities|Casting|CastToCineCameraComponent (Variables|CameraActor|GetCameraComponent)))
    (bind _ascine_camera_component_2 (Utilities|Casting|CastToCineCameraComponent (Variables|/Script/Engine.CameraActor|GetCameraComponent (Utilities|Array|Get(acopy) (Variables|Default|GetAllCameras) (Variables|Default|GetCameraIndex)))))
    (Variables|/Script/CinematicCamera.CineCameraComponent|SetCurrentFocalLength _ascine_camera_component (Variables|/Script/CinematicCamera.CineCameraComponent|GetCurrentFocalLength _ascine_camera_component_2))
    (Utilities|FlowControl|Sequence
      (:then_0
        (bind _outactors (Actor|GetAllActorsOfClass "/Script/ROSIntegrationVision.VisionActor"))
        (Utilities|IsValid (Utilities|Array|Get(acopy) _outactors)
          (:Is%20Valid
            (Transformation|AttachActorToActor (Utilities|Array|Get(acopy) _outactors) 0 "None" "SnapToTarget" "SnapToTarget" "SnapToTarget" true)
            (Variables|/Script/Engine.SceneCaptureComponent2D|SetFOVAngle (Variables|/Script/ROSIntegrationVision.VisionComponent|GetObject (Variables|/Script/ROSIntegrationVision.VisionActor|Getvision (Utilities|Array|Get(acopy) _outactors))) (Variables|/Script/Engine.SceneCaptureComponent2D|GetFOVAngle (Variables|/Script/Composure.CompositingCaptureBase|GetSceneCaptureComponent2D (Variables|Default|GetCompEl))))
            (Transformation|SetWorldTransform (Variables|/Script/ROSIntegrationVision.VisionComponent|GetObject (Variables|/Script/ROSIntegrationVision.VisionActor|Getvision (Utilities|Array|Get(acopy) _outactors))) (Transformation|GetWorldTransform (Variables|CameraActor|GetCameraComponent)) false false))))
      (:then_1
        (bind _outactors_2 (Actor|GetAllActorswithTag "Rain"))
        (Utilities|IsValid (Utilities|Array|Get(acopy) _outactors_2)
          (:Is%20Valid
            (Transformation|SetActorLocation (Utilities|Array|Get(acopy) _outactors_2) (.location (Transformation|GetWorldTransform (Variables|CameraActor|GetCameraComponent))) false true)))))
    (else
      (Utilities|IsValid (Game|GetPlayerCameraManager 0)
        (:Is%20Valid
          (Transformation|SetActorLocationAndRotation (Camera|GetCameraLocation _returnvalue) (Camera|GetCameraRotation _returnvalue))
          (Default|CopyCameraSettingstoSceneCapture (Variables|Default|GetCompEl) (Variables|CameraActor|GetCameraComponent) (Variables|/Script/Composure.CompositingCaptureBase|GetSceneCaptureComponent2D (Variables|Default|GetCompEl))))))))

(fn ConstructionScript)