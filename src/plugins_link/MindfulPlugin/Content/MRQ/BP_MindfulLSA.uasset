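; Level sequence Blueprint that starts a Movie Render Queue render of its sequence on BeginPlay, unless a render is already running.
; After a short delay it trims playback to Duration, allocates a job with the current level and Config, and renders the queue through a new-process executor.
; It binds print-only completion callbacks to a separately constructed PIE executor, which is not the one that runs the render.
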(event Custom|OnJobFinished
  (params (FinishedJob :type Movie%20Pipeline%20Executor%20Job%20Object%20Reference) (bSuccess :type Boolean))
  (Development|PrintString "Job Finished"))

(event Custom|OnJobWorkFinished
  (params (Results :type Movie%20Pipeline%20Output%20Data%20Structure))
  (Development|PrintString "Job Work Finished"))

(event Custom|OnShotWorkFinished
  (params (Results :type Movie%20Pipeline%20Output%20Data%20Structure))
  (Development|PrintString "Shot Finished"))

(event EventBeginPlay
  (if (not (Class|MoviePipelineQueueEngineSubsystem|IsRendering (|MoviePipelineQueueEngineSubsystem)))
    (Utilities|FlowControl|Delay 1.0)
    (bind _returnvalue (Game|ConstructObjectfromClass "/Script/MovieRenderPipelineEditor.MoviePipelinePIEExecutor"))
    (bind _output_get (Variables|Default|SetExecutor _returnvalue))
    (Utilities|FlowControl|Sequence
      (:then_0
        (EventDispatchers|AssignOnIndividualJobFinishedDelegate _output_get (delegate Custom|OnJobFinished))
        (EventDispatchers|AssignOnIndividualJobWorkFinishedDelegate (Variables|Default|GetExecutor) (delegate Custom|OnJobWorkFinished)))
      (:then_1
        (EventDispatchers|AssignOnIndividualShotWorkFinishedDelegate (Variables|Default|GetExecutor) (delegate Custom|OnShotWorkFinished)))
      (:then_2
        (Class|MovieSceneSequenceExtensions|SetPlaybackEnd (Variables|Default|GetLevelSequenceAsset) (Variables|Default|GetDuration))
        (Class|MoviePipelineQueueEngineSubsystem|SetConfiguration (|MoviePipelineQueueEngineSubsystem) 0 true)
        (bind _returnvalue_2 (Class|MoviePipelineQueueEngineSubsystem|AllocateJob (|MoviePipelineQueueEngineSubsystem) (Variables|Default|GetLevelSequenceAsset)))
        (bind _output_get_2 (Variables|Default|SetJob _returnvalue_2))
        (Variables|/Script/MovieRenderPipelineCore.MoviePipelineExecutorJob|SetMap _output_get_2 (Utilities|GetSoftObjectPath (Class|Actor|GetLevel)))
        (Class|MoviePipelineExecutorJob|SetConfiguration (Variables|Default|GetJob) (Variables|Default|GetConfig))
        (Class|MoviePipelineQueueEngineSubsystem|RenderQueuewithExecutor (|MoviePipelineQueueEngineSubsystem) "/Script/MovieRenderPipelineEditor.MoviePipelineNewProcessExecutor")))))

(event Collision|EventActorBeginOverlap
  (params (OtherActor :type Actor%20Object%20Reference)))

(event EventTick
  (params (DeltaSeconds :type Float%20%28single-precision%29)))

(fn ConstructionScript)