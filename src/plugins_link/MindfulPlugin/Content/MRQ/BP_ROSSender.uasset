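; BP_ROSSender is an actor that streams Movie Render Queue frames to ROS as color image and ground truth messages.
; BeginPlay creates the two ROS topics.
; Each Tick checks the saved MovieRenders folder for the current frame's final image and stencil mask PNGs, publishes ground truth from the mask, then the color image.
; The frame Id advances only after both publishes succeed, so missing or failed frames are retried.
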(event EventBeginPlay
  (Development|PrintString "ROS Sender Begin Play")
  (bind _returnvalue (Game|ConstructObjectfromClass "/Script/ROSIntegration.Topic"))
  (bind _output_get (Variables|Default|SetColorTopic _returnvalue))
  (Class|Topic|InitImage _output_get "/unreal_ros/image_color" 1)
  (bind _returnvalue_2 (Game|ConstructObjectfromClass "/Script/ROSIntegration.Topic"))
  (bind _output_get_2 (Variables|Default|SetGroundTruthTopic _returnvalue_2))
  (Class|Topic|Init _output_get_2 "/unreal_ros/ground_truth" "String" 1))

(event Collision|EventActorBeginOverlap
  (params (OtherActor :type Actor%20Object%20Reference)))

(event EventTick
  (params (DeltaSeconds :type Float%20%28single-precision%29))
  (bind _returnvalue (Class|KismetSystemLibrary|GetProjectSavedDirectory))
  (bind _returnvalue_2 (Class|Topic|CheckImagePaths (Utilities|Array|MakeArray (Class|BlueprintPathsLibrary|Combine (Utilities|Array|MakeArray _returnvalue (Utilities|String|Append "MovieRenders/MindfulSceneCaptureLS_" (Class|ROSLib|FormatLevelSequenceFrameNumber (Variables|Default|GetId)) "_FinalImage.png"))) (Class|BlueprintPathsLibrary|Combine (Utilities|Array|MakeArray _returnvalue (Utilities|String|Append "MovieRenders/MindfulSceneCaptureLS_" (Class|ROSLib|FormatLevelSequenceFrameNumber (Variables|Default|GetId)) "_FinalImageMRQ_StencilMask.png"))))))
  (if _returnvalue_2
    (Development|PrintString (Utilities|String|Append "attempting to send " (Class|BlueprintPathsLibrary|Combine (Utilities|Array|MakeArray _returnvalue (Utilities|String|Append "MovieRenders/MindfulSceneCaptureLS_" (Class|ROSLib|FormatLevelSequenceFrameNumber (Variables|Default|GetId)) "_FinalImage.png")))))
    (Development|PrintString (Utilities|String|Append "attempting to send " (Class|BlueprintPathsLibrary|Combine (Utilities|Array|MakeArray _returnvalue (Utilities|String|Append "MovieRenders/MindfulSceneCaptureLS_" (Class|ROSLib|FormatLevelSequenceFrameNumber (Variables|Default|GetId)) "_FinalImageMRQ_StencilMask.png")))))
    (bind _returnvalue_3 (Class|Topic|TestPublishGroundTruthfromPNG (Variables|Default|GetGroundTruthTopic) (Class|BlueprintPathsLibrary|Combine (Utilities|Array|MakeArray _returnvalue (Utilities|String|Append "MovieRenders/MindfulSceneCaptureLS_" (Class|ROSLib|FormatLevelSequenceFrameNumber (Variables|Default|GetId)) "_FinalImageMRQ_StencilMask.png"))) (Variables|Default|GetId)))
    (if _returnvalue_3
      (bind _colortopic (Variables|Default|GetColorTopic)
        (:then
          (bind _returnvalue_4 (Class|Topic|PublishImageMessagefromPNG _colortopic (Class|BlueprintPathsLibrary|Combine (Utilities|Array|MakeArray _returnvalue (Utilities|String|Append "MovieRenders/MindfulSceneCaptureLS_" (Class|ROSLib|FormatLevelSequenceFrameNumber (Variables|Default|GetId)) "_FinalImage.png"))) (Variables|Default|GetId)))
          (if _returnvalue_4
            (Variables|Default|SetId (+ (Variables|Default|GetId) 1))))
        (:else))
      (else
        (Development|PrintString "ROS Sender: Failed to send Ground Truth. Going to try and send this frame again")))
    (else
      (Development|PrintString "ROS Sender: One of the required files doesnt exist yet"))))

(fn ConstructionScript)