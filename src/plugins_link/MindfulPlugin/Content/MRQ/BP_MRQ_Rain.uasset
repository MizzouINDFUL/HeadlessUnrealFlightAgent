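; BP_MRQ_Rain is a rain effect actor that follows the player pawn.
; Every tick it teleports to a point a fixed distance ahead of the pawn along its forward vector, keeping the rain in front of the player.
; The construction script passes the Intensity variable to the VFXRain component's RainIntensity parameter.
; Custom depth rendering is turned off on that component at construction and again on BeginPlay.
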(event EventBeginPlay
  (Rendering|SetRenderCustomDepth (Variables|Default|GetVFX_Rain) false))

(event Collision|EventActorBeginOverlap
  (params (OtherActor :type Actor%20Object%20Reference)))

(event EventTick
  (params (DeltaSeconds :type Float%20%28single-precision%29))
  (bind _returnvalue (Game|Player|GetPlayerPawn 0))
  (Transformation|SetActorLocation (+ (Transformation|GetActorLocation _returnvalue) (* (Transformation|GetActorForwardVector _returnvalue) 5e+02)) false true))

(fn ConstructionScript
  (Niagara|SetNiagaraVariable(Float) (Variables|Default|GetVFX_Rain) "RainIntensity" (Variables|Default|GetIntensity))
  (Rendering|SetRenderCustomDepth (Variables|Default|GetVFX_Rain) false))