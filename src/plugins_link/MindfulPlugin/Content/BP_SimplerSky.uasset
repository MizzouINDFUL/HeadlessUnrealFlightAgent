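; Simple sky actor that draws the sky on a sphere mesh using the M_SimpleSky material.
; The construction script and BeginPlay both create a dynamic instance of that material and set its DayProgress parameter from the Progress variable.
; Tick is unused, so the time of day stays at the set Progress value rather than advancing on its own.
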(event EventBeginPlay
  (bind _returnvalue (Rendering|Material|CreateDynamicMaterialInstance (Variables|Default|GetSphere) 0 "/MindfulPlugin/M_SimpleSky.M_SimpleSky" "None" :!class /Script/Engine.PrimitiveComponent))
  (bind _output_get (Variables|Default|SetDynMat _returnvalue))
  (Rendering|Material|SetScalarParameterValue _output_get "DayProgress" (Variables|Default|GetProgress) :!class /Script/Engine.MaterialInstanceDynamic))

(event Collision|EventActorBeginOverlap
  (params (OtherActor :type Actor%20Object%20Reference)))

(event EventTick
  (params (DeltaSeconds :type Float%20%28single-precision%29)))

(fn ConstructionScript
  (bind _returnvalue (Rendering|Material|CreateDynamicMaterialInstance (Variables|Default|GetSphere) 0 "/MindfulPlugin/M_SimpleSky.M_SimpleSky" "None" :!class /Script/Engine.PrimitiveComponent))
  (bind _output_get (Variables|Default|SetDynMat _returnvalue))
  (Rendering|Material|SetScalarParameterValue _output_get "DayProgress" (Variables|Default|GetProgress) :!class /Script/Engine.MaterialInstanceDynamic)
  (Rendering|Material|SetMaterial (Variables|Default|GetSphere) 0 _output_get))